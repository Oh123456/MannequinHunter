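; BP_Kurumi1 is a character Blueprint with a capsule and skeletal mesh that exposes a weapon socket position and an IK trace distance.
; The construction script derives IKTraceDistance from the scaled capsule half-height multiplied by the actor's Z scale.
; GetWeaponeSocket returns the location of the L_hand socket on SkeletalMesh1.
; The event graph holds only empty BeginPlay, overlap and Tick events.
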(event `self.ReceiveTick`
  (params (DeltaSeconds :type "Float (single-precision)")))

(fn `GetWeaponeSocket`
  (returns (NewParam :type "Vector Structure"))
  (return (`SceneComponent.GetSocketLocation` (`self.SkeletalMesh1`) "L_hand")))

(fn `UserConstructionScript`
  (set `self.Scale` (.z (.scale (`self.GetTransform`))))
  (set `self.IK Trace Distance` (* (`CapsuleComponent.GetScaledCapsuleHalfHeight` (`self.CapsuleComponent`)) (`self.Scale`))))